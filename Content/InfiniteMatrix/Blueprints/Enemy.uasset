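; Enemy actor with a Cube component that scores points when shot and damages the player on contact.
; On Cube overlap, a projectile is destroyed along with the Cube component, and the BP_Player found in the world gains a point.
; Overlap with BP_Player instead subtracts health; at zero or below it flags the player dead, shows the restart screen and resets score.
; The actor itself is never destroyed, only its Cube.
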(event `self.Cube.OnComponentBeginOverlap`
  (params (OverlappedComponent :type "PrimitiveComponent Object Reference") (OtherActor :type "Actor Object Reference") (OtherComp :type "PrimitiveComponent Object Reference") (OtherBodyIndex :type Integer) (bFromSweep :type Boolean) (SweepResult :type "HitResult Structure (by ref)"))
  (bind _asprojectile (cast `/Game/InfiniteMatrix/Blueprints/projectile` OtherActor)
    (:`then`
      (`self.K2_DestroyActor` _asprojectile)
      (`ActorComponent.K2_DestroyComponent` (`self.Cube`))
      (bind _returnvalue (`GameplayStatics.GetActorOfClass` "/Game/InfiniteMatrix/Blueprints/BP_Player.BP_Player_C"))
      (set `/Game/InfiniteMatrix/Blueprints/BP_Player.score` (+ (`/Game/InfiniteMatrix/Blueprints/BP_Player.score` _returnvalue) 1.0) _returnvalue))
    (:`CastFailed`
      (bind _asbp_player (cast `/Game/InfiniteMatrix/Blueprints/BP_Player` OtherActor))
      (bind _output_get (set `/Game/InfiniteMatrix/Blueprints/BP_Player.Health` (- (`/Game/InfiniteMatrix/Blueprints/BP_Player.Health` _asbp_player) 10.0) _asbp_player))
      (if (<= _output_get 0.0)
        (set `/Game/InfiniteMatrix/Blueprints/BP_Player.IsDead` true _asbp_player)
        (`/Game/InfiniteMatrix/Blueprints/BP_Player.DisplayRestart` _asbp_player)
        (set `/Game/InfiniteMatrix/Blueprints/BP_Player.score` 0.0 _asbp_player)))))

(event `self.Cube.OnComponentEndOverlap`
  (params (OverlappedComponent :type "PrimitiveComponent Object Reference") (OtherActor :type "Actor Object Reference") (OtherComp :type "PrimitiveComponent Object Reference") (OtherBodyIndex :type Integer)))

(fn `UserConstructionScript`)